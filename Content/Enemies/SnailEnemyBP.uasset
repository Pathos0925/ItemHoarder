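; Snail enemy that wanders random navmesh points and hunts the player when sighted (if chase is enabled), hit, or flagged as attracting snails.
; Tick drives AI movement, rotates the health widget toward the player, and registers the snail as a damager while angry and overlapping them.
; Projectile overlaps reduce health, update the widget and trigger pursuit; death spawns chance-based loot from a drop map.
; Pursuit shows an alert icon on the widget.
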(event OnSeePawn(PawnSensing)
  (params (Pawn :type Pawn%20Object%20Reference))
  ;[1 1 1] See Player
  (Utilities|Casting|CastToFirstPersonCharacter Pawn)
  (if (Variables|Default|GetChasePlayerInRange)
    (Variables|Default|SetinRange true)
    (Utilities|HuntPlayer)))

(event Custom|FadeOutAlert
  ;[1 1 1] Fade out alert
  (Development|PrintString "playing fadeout" true true "(R=0.000000,G=0.992108,B=1.000000,A=1.000000)")
  (bind _opacity (Timeline|AlertFadeTimeline PlayFromStart)
    (:Update
      (bind _asenemy_health (Utilities|Casting|CastToEnemyHealth (UserInterface|GetUserWidgetObject (Variables|Default|GetHealthWidget))))
      (Default|SetAlertOpacity _asenemy_health _opacity))
    (:Finished)))

(event EventBeginPlay
  ;[1 1 1] Update Widget on start
  (CallFunction|UpdateHealthWidget)
  (bind _asfirst_person_character (Utilities|Casting|CastToFirstPersonCharacter (Game|GetPlayerCharacter 0)))
  (Variables|Default|SetFindPlayerAnywhere (or (Variables|/Game/FirstPersonBP/Blueprints/FirstPersonCharacter.FirstPersonCharacter_C|GetAttractingSnails _asfirst_person_character) (Variables|Default|GetFindPlayerAnywhere))))

(event Collision|EventActorBeginOverlap
  (params (OtherActor :type Actor%20Object%20Reference))
  ;[1 1 1] Hit With Arrow
  (bind _asfirst_person_projectile (Utilities|Casting|CastToFirstPersonProjectile OtherActor))
  (bind _output_get (Variables|Default|SetHealth (- (Variables|Default|GetHealth) (Variables|/Game/FirstPersonBP/Blueprints/FirstPersonProjectile.FirstPersonProjectile_C|GetDamage _asfirst_person_projectile))))
  (if (<= _output_get 0.0)
    (CallFunction|SpawnDrop)
    (Actor|DestroyActor))
  (Variables|Default|SetFindPlayerAnywhere true)
  (CallFunction|UpdateHealthWidget)
  (Variables|Default|SetAngry true))

(event EventTick
  (params (DeltaSeconds :type Float%20%28single-precision%29))
  ;[1 1 1] EventTick
  (Utilities|FlowControl|Sequence
    (:then_0
      (Utilities|AITick))
    (:then_1
      (CallFunction|AimWidgetatPlayer))
    (:then_2
      ;[1 1 1] Damage player if close and angry
      (bind _asfirst_person_character (Utilities|Casting|CastToFirstPersonCharacter (Game|GetPlayerCharacter 0)))
      (if (Collision|IsOverlappingActor _asfirst_person_character :!class /Script/Engine.Actor)
        (if (Variables|Default|GetAngry)
          (bind _asfirst_person_character_2 (Utilities|Casting|CastToFirstPersonCharacter (Game|GetPlayerCharacter 0)))
          (Default|AddDamagerF _asfirst_person_character_2 self))))))

(fn ConstructionScript
  (Variables|Default|SetMaxHealth (Variables|Default|GetHealth))
  (CallFunction|UpdateHealthWidget))

(fn UpdateHealthWidget
  (bind _asenemy_health (Utilities|Casting|CastToEnemyHealth (UserInterface|GetUserWidgetObject (Variables|Default|GetHealthWidget))))
  (Default|SetHealth _asenemy_health (/ (Variables|Default|GetHealth) (Variables|Default|GetMaxHealth)))
  (Default|SetName _asenemy_health (Variables|Default|GetName)))

(fn AimWidgetatPlayer
  (Transformation|SetWorldRotation (Variables|Default|GetHealthWidget) (Math|Rotator|FindLookatRotation (Transformation|GetActorLocation) (.location (Transformation|GetActorTransform (Game|GetPlayerCharacter 0)))) false false))

(fn SpawnDrop
  (bind _possibledrops (Variables|Default|GetPossibleDrops))
  (bind _keys (Utilities|Map|Keys _possibledrops))
  (bind _values (Utilities|Map|Values _possibledrops))
  (for _index (range 0 (- (Utilities|Array|Length _keys) 1))
    (if (>= (.dropchance (Utilities|Array|Get(acopy) _values _index)) (Math|Random|RandomFloat))
      (for _index_2 (range 0 (Math|Random|RandomIntegerinRange (.dropmin (Utilities|Array|Get(acopy) _values _index)) (.dropmax (Utilities|Array|Get(acopy) _values _index))))
        (Game|SpawnActorfromClass (Utilities|Array|Get(acopy) _keys _index) (Transformation|GetActorTransform self) "AdjustIfPossibleButAlwaysSpawn" 0 0)))))

(fn SetAlertImage
  (if (not (Variables|Default|GetAlerted))
    (Variables|Default|SetAlerted true)
    (bind _asenemy_health (Utilities|Casting|CastToEnemyHealth (UserInterface|GetUserWidgetObject (Variables|Default|GetHealthWidget))))
    (Default|SetAlertImage _asenemy_health "/Game/Textures/Alert01.Alert01")))